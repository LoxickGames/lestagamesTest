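; BP_WindPlatform is an obstacle platform whose wind pushes the main character in a randomly changing horizontal direction.
; A looping timer randomly picks one of four axis-aligned states, setting the movement direction, impulse and Niagara wind effect variable.
; Box overlaps cache the BP_MainCharacter and toggle InBlock.
; While InBlock is set, Tick adds movement input and a velocity-change impulse every frame, without delta-time scaling.
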(event OnComponentBeginOverlap(Box)
  (params (OverlappedComponent :type Primitive%20Component%20Object%20Reference) (OtherActor :type Actor%20Object%20Reference) (OtherComp :type Primitive%20Component%20Object%20Reference) (OtherBodyIndex :type Integer) (bFromSweep :type Boolean) (SweepResult :type Hit%20Result%20Structure%20%28by%20ref%29))
  (bind _asbp_main_character (Utilities|Casting|CastToBP_MainCharacter OtherActor))
  (Variables|Default|SetAs%20BP%20Main%20Character _asbp_main_character)
  (Variables|Default|SetInBlock true))

(event OnComponentEndOverlap(Box)
  (params (OverlappedComponent :type Primitive%20Component%20Object%20Reference) (OtherActor :type Actor%20Object%20Reference) (OtherComp :type Primitive%20Component%20Object%20Reference) (OtherBodyIndex :type Integer))
  (Utilities|Casting|CastToBP_MainCharacter OtherActor)
  (Variables|Default|SetInBlock false))

(event Custom|SetDirection
  (Variables|Default|SetStateRotation (.OutItem (Utilities|Array|Random (Utilities|Array|MakeArray "NewEnumerator0" "NewEnumerator1" "NewEnumerator2" "NewEnumerator3"))))
  (switch Utilities|FlowControl|Switch|SwitchonEN_WindState (Variables|Default|GetStateRotation)
    (:NewEnumerator0
      (Variables|Default|SetWorld%20Direction "1.000000,0.000000,0.000000")
      (Variables|Default|SetImpulse "5.000000,0.000000,0.000000")
      (Niagara|SetNiagaraVariable(Vector3) (Variables|Default|GetNS_WindSwish) "Wind Direction" "0.000000,0.000000,0.000000"))
    (:NewEnumerator1
      (Variables|Default|SetWorld%20Direction "-1.000000,0.000000,0.000000")
      (Variables|Default|SetImpulse "-5.000000,0.000000,0.000000")
      (Niagara|SetNiagaraVariable(Vector3) (Variables|Default|GetNS_WindSwish) "Wind Direction" "-20.000000,0.000000,0.000000"))
    (:NewEnumerator2
      (Variables|Default|SetWorld%20Direction "0.000000,1.000000,0.000000")
      (Variables|Default|SetImpulse "0.000000,5.000000,0.000000")
      (Niagara|SetNiagaraVariable(Vector3) (Variables|Default|GetNS_WindSwish) "Wind Direction" "-20.000000,20.000000,0.000000"))
    (:NewEnumerator3
      (Variables|Default|SetWorld%20Direction "0.000000,-1.000000,0.000000")
      (Variables|Default|SetImpulse "0.000000,-5.000000,0.000000")
      (Niagara|SetNiagaraVariable(Vector3) (Variables|Default|GetNS_WindSwish) "Wind Direction" "-20.000000,-20.000000,0.000000"))))

(event EventBeginPlay
  (Utilities|Time|SetTimerbyEvent (delegate Custom|SetDirection) 2.0 true))

(event Collision|EventActorBeginOverlap
  (params (OtherActor :type Actor%20Object%20Reference)))

(event EventTick
  (params (DeltaSeconds :type Float%20%28single-precision%29))
  (bind _as_bp_main_character (Variables|Default|GetAs%20BP%20Main%20Character))
  (if (Variables|Default|GetInBlock)
    (Pawn|Input|AddMovementInput _as_bp_main_character (Variables|Default|GetWorld%20Direction) 0.5 false)
    (Physics|AddImpulse (Variables|/Script/Engine.Character|GetCharacterMovement _as_bp_main_character) (Variables|Default|GetImpulse) true)))

(fn ConstructionScript)