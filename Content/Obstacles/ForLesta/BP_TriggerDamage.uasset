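; BP_TriggerDamage is an obstacle floor panel that damages player characters standing on it after a color-change warning.
; A BP_MainCharacter entering the Box fires a DoOnce-gated timeline that animates FloorColor on a dynamic material, then applies damage to every overlapping character.
; After a short delay a second timeline animates the color again and re-arms the gate, so another hit requires a new begin overlap.
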(event OnComponentBeginOverlap(Box)
  (params (OverlappedComponent :type Primitive%20Component%20Object%20Reference) (OtherActor :type Actor%20Object%20Reference) (OtherComp :type Primitive%20Component%20Object%20Reference) (OtherBodyIndex :type Integer) (bFromSweep :type Boolean) (SweepResult :type Hit%20Result%20Structure%20%28by%20ref%29))
  (Utilities|Casting|CastToBP_MainCharacter OtherActor)
  (CallFunction|EventDamage))

(event Custom|EventDamage
  (Utilities|FlowControl|DoOnce false
    (:Completed
      (bind _newtrack_0 (Timeline|Timeline PlayFromStart)
        (:Update
          (Rendering|Material|SetVectorParameterValue (Variables|Default|GetMaterialInst) "FloorColor" _newtrack_0 :!class /Script/Engine.MaterialInstanceDynamic))
        (:Finished
          (CallFunction|DamageAllPlayers)
          (CallFunction|TimerResetDamage))))))

(event Custom|DamageAllPlayers
  (for _array_element (Collision|GetOverlappingActors (Variables|Default|GetBox) "/Game/Blueprint/BP_MainCharacter.BP_MainCharacter_C" :!class /Script/Engine.PrimitiveComponent)
    (Game|Damage|ApplyDamage _array_element 0.25 0 0)))

(event Custom|ResetDamage
  (Utilities|FlowControl|DoOnce false) ; enters at Reset
)

(event Custom|TimerResetDamage
  (Utilities|FlowControl|Delay 0.5)
  (bind _newtrack_0 (Timeline|Timeline_0 PlayFromStart)
    (:Update
      (Rendering|Material|SetVectorParameterValue (Variables|Default|GetMaterialInst) "FloorColor" _newtrack_0 :!class /Script/Engine.MaterialInstanceDynamic))
    (:Finished
      (CallFunction|ResetDamage))))

(event EventBeginPlay
  (bind _returnvalue (Rendering|Material|CreateDynamicMaterialInstance "/Game/FunObstacleCourse/Mesh/Materials/M_TriggerDamage_Inst.M_TriggerDamage_Inst" "None" "None" :!class /Script/Engine.KismetMaterialLibrary))
  (Variables|Default|SetMaterialInst _returnvalue)
  (Rendering|Material|SetMaterial (Variables|Default|GetSM_FloorPanel_1) 0 _returnvalue))

(fn ConstructionScript)