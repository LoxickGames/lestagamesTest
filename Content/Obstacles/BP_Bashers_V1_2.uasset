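; Basher obstacle with pillars that slide and knock the main character away on contact.
; On BeginPlay, two timelines each drive the relative Y position of one pillar, at opposite fixed X offsets.
; Hit events on four pillar components feed a shared bump event, which casts to BP_MainCharacter and applies a large movement impulse opposite the hit normal.
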(event OnComponentHit(Pillar_21)
  (params (HitComponent :type Primitive%20Component%20Object%20Reference) (OtherActor :type Actor%20Object%20Reference) (OtherComp :type Primitive%20Component%20Object%20Reference) (NormalImpulse :type Vector :default "0, 0, 0") (Hit :type Hit%20Result%20Structure%20%28by%20ref%29))
  (CallFunction|EventBump OtherActor (.Normal (Collision|BreakHitResult Hit))))

(event OnComponentHit(Pillar_23)
  (params (HitComponent :type Primitive%20Component%20Object%20Reference) (OtherActor :type Actor%20Object%20Reference) (OtherComp :type Primitive%20Component%20Object%20Reference) (NormalImpulse :type Vector :default "0, 0, 0") (Hit :type Hit%20Result%20Structure%20%28by%20ref%29))
  (CallFunction|EventBump OtherActor (.Normal (Collision|BreakHitResult Hit))))

(event OnComponentHit(Pillar_2)
  (params (HitComponent :type Primitive%20Component%20Object%20Reference) (OtherActor :type Actor%20Object%20Reference) (OtherComp :type Primitive%20Component%20Object%20Reference) (NormalImpulse :type Vector :default "0, 0, 0") (Hit :type Hit%20Result%20Structure%20%28by%20ref%29))
  (CallFunction|EventBump OtherActor (.Normal (Collision|BreakHitResult Hit))))

(event OnComponentHit(Pillar_22)
  (params (HitComponent :type Primitive%20Component%20Object%20Reference) (OtherActor :type Actor%20Object%20Reference) (OtherComp :type Primitive%20Component%20Object%20Reference) (NormalImpulse :type Vector :default "0, 0, 0") (Hit :type Hit%20Result%20Structure%20%28by%20ref%29))
  (CallFunction|EventBump OtherActor (.Normal (Collision|BreakHitResult Hit))))

(event Custom|EventBump
  (params (Actor :type Actor%20Object%20Reference) (NewParam :type Vector))
  (bind _asbp_main_character (Utilities|Casting|CastToBP_MainCharacter Actor))
  (Physics|AddImpulse (Variables|/Script/Engine.Character|GetCharacterMovement _asbp_main_character) (* NewParam -100000) false))

(event EventBeginPlay
  (Utilities|FlowControl|Sequence
    (:then_0
      (bind _location (Timeline|Pillar1_Location PlayFromStart)
        (:Update
          (Transformation|SetRelativeLocation (Variables|Default|GetPillar_2) (Math|Vector|MakeVector -1e+02 _location 0.0) false false))))
    (:then_2
      (bind _location_2 (Timeline|Pillar3_Location PlayFromStart)
        (:Update
          (Transformation|SetRelativeLocation (Variables|Default|GetPillar_22) (Math|Vector|MakeVector 1e+02 _location_2 0.0) false false))))))

(fn ConstructionScript)