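; BP_Pusher_v1 is an obstacle with a pillar that moves along relative Z and shoves the main character on hit.
; From BeginPlay, the PushSpeed timeline scales the Pusher timeline's play rate by PusherSpeed and calls PlayFromStart on it every update.
; The Pusher timeline drives the pillar's height.
; Hits apply a horizontal movement impulse derived from the negated, scaled world-space impact point, rather than a hit direction.
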(event OnComponentHit(Pillar_1)
  (params (HitComponent :type Primitive%20Component%20Object%20Reference) (OtherActor :type Actor%20Object%20Reference) (OtherComp :type Primitive%20Component%20Object%20Reference) (NormalImpulse :type Vector :default "0, 0, 0") (Hit :type Hit%20Result%20Structure%20%28by%20ref%29))
  (bind _asbp_main_character (Utilities|Casting|CastToBP_MainCharacter OtherActor))
  (Physics|AddImpulse (Variables|/Script/Engine.Character|GetCharacterMovement _asbp_main_character) (* (.impactpoint Hit) "-25.000000,-25.000000,0.000000") false))

(event EventBeginPlay
  (bind _speed (Timeline|PushSpeed PlayFromStart)
    (:Update
      (Components|Timeline|SetPlayRate (Variables|Default|GetPusher) (* _speed (Variables|Default|GetPusherSpeed)))
      (bind _location (Timeline|Pusher PlayFromStart)
        (:Update
          (Transformation|SetRelativeLocation (Variables|Default|GetPillar_1) (Math|Vector|MakeVector 0.0 0.0 _location) false false))))))

(fn ConstructionScript)